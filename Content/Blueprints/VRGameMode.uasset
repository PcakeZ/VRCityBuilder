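; VR game mode that runs the economy of a nuclear-power city-management game, including win, loss and saved high scores.
; A delayed Tick rebuilds totals from data tables and interface messages, then updates money, population, research, power, radiation and health.
; Timed random events and upgrades modify these stats, and day/night changes relay through interfaces.
; Excess radiation ends the game, while launching waste by rocket wins and records current radiation as score.
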(event `self.ReceiveBeginPlay`
  (`KismetSystemLibrary.ExecuteConsoleCommand` "\"Stereo on\"" null)
  (`KismetSystemLibrary.ExecuteConsoleCommand` "Stereo on" null)
  ;[1 1 1] Set needed Values
  (`KismetSystemLibrary.Delay` 0.2)
  (bind _asvrpawn (cast `/Game/Blueprints/VRPawn` (`GameplayStatics.GetPlayerPawn` 0)))
  (set `self.PlayerPawn` _asvrpawn)
  (set `self.CurrentRandEventTime` (`KismetMathLibrary.RandomFloatInRange` (`self.RandEventMinTime`) (`self.RandEventMaxTime`)))
  (`self.LoadScore`))

(event `self.ReceiveTick`
  (params (DeltaSeconds :type "Float (single-precision)"))
  (`KismetSystemLibrary.Delay` (`self.CallDelay`))
  (`|ExecutionSequence`
    (:`then_0`
      ;[1 1 1] Get powerplant Values
      (bind _returnvalue (`|GetDataTableRow` "/Game/Blueprints/DataManagement/DT_Powerplant.DT_Powerplant" (`KismetStringLibrary.Conv_StringToName` (`KismetStringLibrary.Concat_StrStr` "Powerplant" (`KismetStringLibrary.Conv_IntToString` (`self.PowerStationLevel`)))))
        (:`then`
          (bind (_maxpower _wasteefficiency _powerefficiency _price _populationrequired _wastebarrelsize _dailyrunningcosts) (break `/Game/Blueprints/DataManagement/Struct_Powerplant` _returnvalue))
          (set `self.WasteEfficiency` _wasteefficiency)
          (set `self.PowerEfficiency` _powerefficiency)
          (set `self.PowerplantCosts` _dailyrunningcosts)
          (`self.ResetValues`)
          ;[1 1 1] Set adds the building bonuses to the values
          (`self.SetValues`)
          (bind _outactors (`GameplayStatics.GetAllActorsWithInterface` "/Game/Blueprints/Interface/I_Storage.I_Storage_C"))
          (for _array_element _outactors
            (message `/Game/Blueprints/Interface/I_Storage.GetStorage` _array_element))
          (bind _outactors_2 (`GameplayStatics.GetAllActorsWithInterface` "/Game/Blueprints/Interface/I_NuclearWaste.I_NuclearWaste_C"))
          (for _array_element_2 _outactors_2
            (message `/Game/Blueprints/Interface/I_NuclearWaste.GetUnstoredWaste` _array_element_2))
          (set `self.TotalWaste` (+ (`self.UnstoredWaste`) (`self.WasteStored`))))))
    (:`then_1`
      (`self.RemoveBuildingBonus`)
      ;[1 1 1] Sets the values for each resource
      (`self.SetMoney`)
      (`self.SetPopulation`)
      (`self.SetResearch`)
      (`self.SetRadition`)
      (`self.SetPower`)
      (`self.SetPopulationHealth`)
      (set `self.CurrentRandEventTime` (- (`self.CurrentRandEventTime`) (`self.CallDelay`)))
      (bind _returnvalue_2 (`GameplayStatics.GetCurrentLevelName` true))
      (if (and (<= (`self.CurrentRandEventTime`) 0.0) (`KismetStringLibrary.NotEqual_StrStr` _returnvalue_2 "MainMenu"))
        (if (not (`self.RandomEventActive`))
          (`self.StartRandomEvent`)
          (set `self.RandomEventActive` true))))))

(event `/Game/Blueprints/Interface/I_NightDayCall.DayStart`
  ;[1 1 1] On Day Start
  (bind _outactors (`GameplayStatics.GetAllActorsWithInterface` "/Game/Blueprints/Interface/I_NightDayCall.I_NightDayCall_C"))
  (for _array_element _outactors
    (if (!= _array_element self)
      (message `/Game/Blueprints/Interface/I_NightDayCall.DayStart` _array_element))))

(event `/Game/Blueprints/Interface/I_RandomEvent.EventEnd`
  (params (Option1Chosen :type Boolean))
  (bind _currenteventname (`self.CurrentEventName`))
  ;[1 1 1] Apply random event values
  (set `self.RandomEventActive` false)
  (if Option1Chosen
    (switch `name` _currenteventname
      (:`RadiationLeak`
        (set `self.Money` (- (`self.Money`) 250.0)))
      (:`ForScience`
        (set `self.ResearchBuildingBonus` (+ (`self.ResearchBuildingBonus`) 1.0))
        (set `self.Money` (- (`self.Money`) 1500.0)))
      (:`MorePower`
        (set `self.ActiveRadiation` (+ (`self.ActiveRadiation`) 20.0)))
      (:`Money!`
        (set `self.Money` (+ (`self.Money`) 1000.0))
        (set `self.Population` (- (`self.Population`) 50.0))))
    (set `self.CurrentRandEventTime` (`KismetMathLibrary.RandomFloatInRange` (`self.RandEventMinTime`) (`self.RandEventMaxTime`)))
    (else
      (switch `name` _currenteventname
        (:`RadiationLeak`
          (set `self.BaseRadiation` (+ (`self.BaseRadiation`) 20.0)))
        (:`ForScience`
          (set `self.Money` (+ (`self.Money`) 1500.0)))
        (:`MorePower`
          (set `self.Population` (- (`self.Population`) 25.0)))
        (:`Money!`
          (set `self.Population` (+ (`self.Population`) 35.0))))
      (set `self.CurrentRandEventTime` (`KismetMathLibrary.RandomFloatInRange` (`self.RandEventMinTime`) (`self.RandEventMaxTime`))))))

(event `/Game/Blueprints/Interface/I_NightDayCall.NightStart`
  ;[1 1 1] On Night Start
  (bind _outactors (`GameplayStatics.GetAllActorsWithInterface` "/Game/Blueprints/Interface/I_NightDayCall.I_NightDayCall_C"))
  (for _array_element _outactors
    (if (!= _array_element self)
      (message `/Game/Blueprints/Interface/I_NightDayCall.NightStart` _array_element))))

(event `/Game/Blueprints/Interface/I_ResearchUpgrade.PopulationBoost`
  ;[1 1 1] Upgrades
  (set `self.UpPopCapMulti` (+ 0.2 (`self.UpPopCapMulti`))))

(event `/Game/Blueprints/Interface/I_ResearchUpgrade.ResearchBoost`
  ;[1 1 1] Upgrades
  (set `self.UpResearchMulti` (+ 0.2 (`self.UpResearchMulti`))))

(event `/Game/Blueprints/Interface/I_ResearchUpgrade.MoneyBoost`
  ;[1 1 1] Upgrades
  (set `self.Money` (+ 2000.0 (`self.Money`))))

(event `/Game/Blueprints/Interface/I_ResearchUpgrade.ShoppingBoost`
  ;[1 1 1] Upgrades
  (set `self.UpShoppingMulti` (+ 0.2 (`self.UpShoppingMulti`))))

(event `/Game/Blueprints/Interface/I_ResearchUpgrade.WasteBoost`
  ;[1 1 1] Upgrades
  (set `self.UpStorageMulti` (+ 0.2 (`self.UpStorageMulti`)))
  (bind _outactors (`GameplayStatics.GetAllActorsWithInterface` "/Game/Blueprints/Interface/I_Storage.I_Storage_C"))
  (for _array_element _outactors
    (message `/Game/Blueprints/Interface/I_Storage.StorageUpgrade` _array_element)))

(event `/Game/Blueprints/Interface/I_ResearchUpgrade.PowerBoost`
  ;[1 1 1] Upgrades
  (set `self.UpWatseMulti` (* (`self.UpWatseMulti`) 0.5)))

(event `/Game/Blueprints/Interface/I_ResearchUpgrade.RocketWasteManagement`
  ;[1 1 1] Upgrades
  (`self.RocketLaunch`)
  (`self.AddScore` (`self.CurrentRadiation`))
  (`KismetSystemLibrary.Delay` 15.0)
  (`/Game/Blueprints/Interface/I_Player.GameOver` (`self.PlayerPawn`) "You Win!" "You launched all your uranium waste to space! It's now someone elses problem!"))

(fn `AddScore`
  (params (Score :type "Float (double-precision)"))
  (locals (NewScore :type "Float (double-precision)") (ScoreSlot :type Integer :default 10))
  (bind _scoreslot (`local.ScoreSlot`))
  (set `self.Score` Score)
  (set `local.NewScore` Score)
  (bind (_arrayindex _arrayelement) (`/Engine/EditorBlueprintResources/StandardMacros.ReverseForEachLoop` (`self.HighScore`))
    (:`LoopBody`
      (if (> _arrayelement (`local.NewScore`))
        (set `local.ScoreSlot` _arrayindex)))
    (:`Completed`
      (if (< (`local.ScoreSlot`) 10)
        (bind _arrayindex_2 (`/Engine/EditorBlueprintResources/StandardMacros.ReverseForEachLoop` (`self.HighScore`))
          (:`LoopBody`
            (if (> _arrayindex_2 (`local.ScoreSlot`))
              (`KismetArrayLibrary.Array_Set` (`self.HighScore`) _arrayindex_2 (`|GetArrayItem` (`self.HighScore`) (- _arrayindex_2 1)))))
          (:`Completed`
            (`KismetArrayLibrary.Array_Set` (`self.HighScore`) _scoreslot (`local.NewScore`))
            (set `self.HighScoreLevel` _scoreslot)
            (bind _returnvalue (`GameplayStatics.CreateSaveGameObject` "/Game/Blueprints/MySaveGame.MySaveGame_C"))
            (set `/Game/Blueprints/MySaveGame.HighScores` (`self.HighScore`) _returnvalue)
            (set `/Game/Blueprints/MySaveGame.Score` (`local.NewScore`) _returnvalue)
            (set `/Game/Blueprints/MySaveGame.HighScoreLevel` (`self.HighScoreLevel`) _returnvalue)
            (set `/Game/Blueprints/MySaveGame.Active` true _returnvalue)
            (`GameplayStatics.SaveGameToSlot` _returnvalue "SaveSlot")))))))

(fn `ApplyEvent`
  (params (ValueName :type String) (ValueAmount :type "Float (double-precision)"))
  (switch `string` ValueName
    (:`Money`
      (set `self.Money` (+ ValueAmount (`self.Money`))))
    (:`Population`
      (set `self.Population` (+ ValueAmount (`self.Population`))))
    (:`NuclearWaste`
      (set `self.TotalWaste` (+ ValueAmount (`self.TotalWaste`))))
    (:`Research`
      (set `self.Research` (+ ValueAmount (`self.Research`))))
    (:`Radiation`
      (set `self.BaseRadiation` (+ ValueAmount (`self.BaseRadiation`))))
    (:`PopulationHealth`
      (set `self.PopulationHealth` (+ ValueAmount (`self.PopulationHealth`))))))

(fn `DebugPrintValues`
  (`KismetSystemLibrary.PrintString` (`KismetStringLibrary.Concat_StrStr` "Pop " (`KismetStringLibrary.Conv_IntToString` (`KismetMathLibrary.Round` (`self.Population`))) " / " (`KismetStringLibrary.Conv_IntToString` (`KismetMathLibrary.Round` (`self.PopulationCap`)))))
  (`KismetSystemLibrary.PrintString` (`KismetStringLibrary.Concat_StrStr` "Research  " (`KismetStringLibrary.Conv_DoubleToString` (`self.Research`))))
  (`KismetSystemLibrary.PrintString` (`KismetStringLibrary.Concat_StrStr` "Money $" (`KismetStringLibrary.Conv_DoubleToString` (`self.Money`))))
  (`KismetSystemLibrary.PrintString` (`KismetStringLibrary.Concat_StrStr` "Raditation " (`KismetStringLibrary.Conv_DoubleToString` (`self.BaseRadiation`))))
  (`KismetSystemLibrary.PrintString` (`KismetStringLibrary.Concat_StrStr` "Storage " (`KismetStringLibrary.Conv_IntToString` (`KismetMathLibrary.Round` (`self.TotalWaste`))) "/" (`KismetStringLibrary.Conv_DoubleToString` (`self.StorageMax`))))
  (`KismetSystemLibrary.PrintString` (`KismetStringLibrary.Concat_StrStr` "Population Health " (`KismetStringLibrary.Conv_IntToString` (`KismetMathLibrary.Round` (* (`self.PopulationHealth`) 100.0))) "%")))

(fn `LoadScore`
  (if true
    (bind _returnvalue (`GameplayStatics.LoadGameFromSlot` "SaveSlot"))
    (bind _asmy_save_game (cast `/Game/Blueprints/MySaveGame` _returnvalue))
    (set `self.HighScore` (`/Game/Blueprints/MySaveGame.HighScores` _asmy_save_game))
    (set `self.HighScoreLevel` (`/Game/Blueprints/MySaveGame.HighScoreLevel` _asmy_save_game))
    (if (`/Game/Blueprints/MySaveGame.Active` _asmy_save_game)
      (set `self.Score` (`/Game/Blueprints/MySaveGame.Score` _asmy_save_game))
      (bind _returnvalue_2 (`GameplayStatics.CreateSaveGameObject` "/Game/Blueprints/MySaveGame.MySaveGame_C"))
      (set `/Game/Blueprints/MySaveGame.Active` false _returnvalue_2)
      (set `/Game/Blueprints/MySaveGame.HighScores` (`self.HighScore`) _returnvalue_2)
      (set `/Game/Blueprints/MySaveGame.Score` (`self.Score`) _returnvalue_2)
      (set `/Game/Blueprints/MySaveGame.HighScoreLevel` (`self.HighScoreLevel`) _returnvalue_2)
      (`GameplayStatics.SaveGameToSlot` _returnvalue_2 "SaveSlot"))))

(fn `RemoveBuildingBonus`
  (if (not (`self.CityPowered`))
    (set `self.PopulationHealthBuildings` 1.0)))

(fn `ResetValues`
  (set `self.PopulationCap` 0.0)
  (set `self.PowerRequired` 0.0)
  (set `self.PopulationHealthBuildings` 0.0)
  (set `self.StorageMax` 0.0)
  (set `self.WasteStored` 0.0)
  (set `self.MoneyBuildings` 0.0)
  (set `self.ResearchBuildingBonus` 0.0)
  (set `self.UnstoredWaste` 0.0))

(fn `RocketLaunch`
  (bind _outactors (`GameplayStatics.GetAllActorsOfClass` "/Game/Blueprints/Actors/BP_LaunchPad.BP_LaunchPad_C"))
  (`/Game/Blueprints/Actors/BP_LaunchPad.LaunchRocket` (`|GetArrayItem` _outactors)))

(fn `SetMoney`
  (locals (MoneyPerDay :type "Float (double-precision)"))
  (if (`self.CityPowered`)
    (bind _output_get (set `local.MoneyPerDay` (- (* (+ (* (`self.Population`) (`self.StorePopMod`)) (`self.MoneyBuildings`)) (`self.MoneyMultiplier`) (`self.UpShoppingMulti`)) (`self.PowerplantCosts`))))
    (set `self.CurrentMoneyOutput` _output_get)
    (set `self.Money` (+ (/ (`local.MoneyPerDay`) (/ (`self.DaySpeed`) (`self.CallDelay`))) (`self.Money`)))))

(fn `SetPopulation`
  (locals (PopulationPerDay :type "Float (double-precision)"))
  (set `local.PopulationPerDay` (`KismetMathLibrary.FClamp` (* (`self.PopulationMultiplier`) (+ (/ (`self.PopulationCap`) (`self.Population`)) 1.0)) -100.0 100.0))
  (set `self.Population` (`KismetMathLibrary.FClamp` (+ (/ (`local.PopulationPerDay`) (/ (`self.DaySpeed`) (`self.CallDelay`))) (`self.Population`)) 1.0 (`self.PopulationCap`))))

(fn `SetPopulationHealth`
  (locals (PopulationHealthPerDay :type "Float (double-precision)"))
  (set `local.PopulationHealthPerDay` (/ (- (`self.CurrentRadiation`) (`self.PopulationHealthBuildings`)) (`self.PopulationHealthMaxRad`)))
  (bind _output_get (set `self.CurrentHealth` (+ (/ (`local.PopulationHealthPerDay`) (/ (`self.DaySpeed`) (`self.CallDelay`))) (`self.CurrentHealth`))))
  (set `self.PopulationHealth` (/ _output_get (`self.PopulationHealthMaxRad`))))

(fn `SetPower`
  (set `self.PowerRequired` (+ (`self.PowerRequired`) (* (`self.Population`) (`self.PowerPerPerson`))))
  (set `self.CurrentPowerDraw` (/ (* (+ (`self.PowerRequired`) (`self.Population`)) (`self.PowerDrawMultiplier`) (`self.PowerEfficiency`)) (/ (`self.DaySpeed`) (`self.CallDelay`)))))

(fn `SetRadition`
  (set `self.BaseRadiation` (- (* (+ (* (`self.WasteStored`) (`self.StoredRadiationLeakMod`)) (* (`self.RiverWaste`) 0.5)) (`self.RadiationMultiplier`)) (`self.PopulationHealthBuildings`)))
  (set `self.ActiveRadiation` (`self.UnstoredWaste`))
  (bind _output_get (set `self.CurrentRadiation` (`KismetMathLibrary.FClamp` (+ (`self.CurrentRadiation`) (/ (- (+ (`self.ActiveRadiation`) (`self.BaseRadiation`)) (`self.CurrentRadiation`)) (/ (`self.DaySpeed`) (`self.CallDelay`)))) 0.0 (`self.GameoverRadiation`))))
  (bind _returnvalue (/ _output_get (`self.GameoverRadiation`)))
  (if (>= _returnvalue 1.0)
    (`/Game/Blueprints/Interface/I_Player.GameOver` (`self.PlayerPawn`) "Radiation Death" "Radiation levels are too high, we must evacuate the town. The environment is dead.")
    (elif (< _returnvalue (`|GetArrayItem` (`self.Environment`)))
      (set `self.EnvironmentState` "NewEnumerator0")
      (elif (and (< _returnvalue (`|GetArrayItem` (`self.Environment`) 1)) (> _returnvalue (`|GetArrayItem` (`self.Environment`))))
        (set `self.EnvironmentState` "NewEnumerator1")
        (elif (and (< _returnvalue (`|GetArrayItem` (`self.Environment`) 2)) (> _returnvalue (`|GetArrayItem` (`self.Environment`) 1)))
          (set `self.EnvironmentState` "NewEnumerator2")
          (else
            (set `self.EnvironmentState` "NewEnumerator3")))))))

(fn `SetResearch`
  (locals (ResearchPerDay :type "Float (double-precision)"))
  (if (`self.CityPowered`)
    (set `local.ResearchPerDay` (* (`self.ResearchBuildingBonus`) (`self.ResearchMultiplier`) (`self.UpResearchMulti`)))
    (set `self.Research` (+ (/ (`local.ResearchPerDay`) (/ (`self.DaySpeed`) (`self.CallDelay`))) (`self.Research`)))))

(fn `SetValues`
  (for _array_element (`self.AllBuildings`)
    (bind _returnvalue (`|GetDataTableRow` "/Game/Blueprints/DataManagement/DT_BuildingInfo.DT_BuildingInfo" _array_element)
      (:`then`
        (bind (_price _name _level _moneyprovided _powerrequired _populationprovided _researchprovided _storageprovided _radiationreduction _populationhealth) (break `/Game/Blueprints/DataManagement/Struct_Buildings` _returnvalue))
        (set `self.MoneyBuildings` (+ _moneyprovided (`self.MoneyBuildings`)))
        (set `self.PowerRequired` (+ _powerrequired (`self.PowerRequired`)))
        (set `self.PopulationCap` (* (+ _populationprovided (`self.PopulationCap`)) (`self.UpPopCapMulti`)))
        (set `self.ResearchBuildingBonus` (+ _researchprovided (`self.ResearchBuildingBonus`)))
        (set `self.PopulationHealthBuildings` (+ _populationhealth (`self.PopulationHealthBuildings`))))
      (:`RowNotFound`
        (`KismetSystemLibrary.PrintString` "-------- Data Table Row Not Found --------"))))
  (return))

(fn `StartRandomEvent`
  ;[1 1 1] Get Random Row
  (bind _outrownames (`DataTableFunctionLibrary.GetDataTableRowNames` "/Game/Blueprints/DataManagement/DT_RandomEvents.DT_RandomEvents"))
  ;[1 1 1] Activate randomevent widget
  (`/Engine/EditorBlueprintResources/StandardMacros.IsValid` (`self.PlayerPawn`)
    (:`Is Valid`
      (bind _output_get (set `self.CurrentEventName` (`|GetArrayItem` _outrownames (`KismetMathLibrary.RandomIntegerInRange` 0 (- (`KismetArrayLibrary.Array_Length` _outrownames) 1)))))
      (`/Game/Blueprints/Interface/I_RandomEvent.EventBegin` (`self.PlayerPawn`) _output_get))))

(fn `UserConstructionScript`)