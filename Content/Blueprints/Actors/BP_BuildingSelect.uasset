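; VR building picker: a looping horizontal carousel of five building-type rows, each with a vertically scrolling level column.
; While the VR pawn holds build, controller speed drags the rows and selected column; on release they coast with lerped decay, then ease onto the nearest snap point.
; Each tick the row near the centre becomes visible and sets building type and level.
; Rows wrap at the edges, while columns clamp between end levels.
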(event `self.ReceiveBeginPlay`
  (bind _rows (`self.rows`))
  (bind _buildingsnappoints (`self.BuildingSnapPoints`))
  (bind _levelsnappoints (`self.LevelSnapPoints`))
  (`KismetArrayLibrary.Array_Add` _rows (`self.Housing Selected`))
  (`KismetArrayLibrary.Array_Add` _rows (`self.Storage Selected`))
  (`KismetArrayLibrary.Array_Add` _rows (`self.Shops Selected`))
  (`KismetArrayLibrary.Array_Add` _rows (`self.Clinic Selected`))
  (`KismetArrayLibrary.Array_Add` _rows (`self.Research Selected`))
  (`KismetArrayLibrary.Array_Add` _buildingsnappoints (`self.Pos1`))
  (`KismetArrayLibrary.Array_Add` _buildingsnappoints (`self.Pos2`))
  (`KismetArrayLibrary.Array_Add` _buildingsnappoints (`self.Pos3`))
  (`KismetArrayLibrary.Array_Add` _buildingsnappoints (`self.Pos4`))
  (`KismetArrayLibrary.Array_Add` _buildingsnappoints (`self.Pos5`))
  (`KismetArrayLibrary.Array_Add` _levelsnappoints (`self.PosLevel1`))
  (`KismetArrayLibrary.Array_Add` _levelsnappoints (`self.PosLevel2`))
  (`KismetArrayLibrary.Array_Add` _levelsnappoints (`self.PosLevel3`))
  (`KismetArrayLibrary.Array_Add` _levelsnappoints (`self.PosLevel4`))
  (bind _asvrpawn (cast `/Game/Blueprints/VRPawn` (`GameplayStatics.GetPlayerPawn` 0)))
  (set `self.VRPawn` _asvrpawn))

(event `self.ReceiveTick`
  (params (DeltaSeconds :type "Float (single-precision)"))
  (bind _vrpawn (`self.VRPawn`))
  (bind _controllerspeedh (`/Game/Blueprints/VRPawn.ControllerSpeedH` _vrpawn))
  (bind _controllerspeedv (`/Game/Blueprints/VRPawn.ControllerSpeedV` _vrpawn))
  (`|ExecutionSequence`
    (:`then_0`
      (if (`/Game/Blueprints/VRPawn.BuildHeld` (`self.VRPawn`))
        (`SceneComponent.K2_AddRelativeLocation` (`self.rows`) (`KismetMathLibrary.MakeVector` _controllerspeedh) false false)
        (bind _newparam (`self.TestLevelRowHeight`))
        (if _newparam
          (`SceneComponent.K2_AddRelativeLocation` (`self.SelectedRowLevels`) (`KismetMathLibrary.MakeVector` 0.0 0.0 _controllerspeedv) false false))
        (set `self.SpeedH` _controllerspeedh)
        (set `self.SpeedV` _controllerspeedv)
        (`self.TeleportRows`)
        (else
          (if (>= (`KismetMathLibrary.Abs` (`self.SpeedH`)) 0.5)
            (`SceneComponent.K2_AddRelativeLocation` (`self.rows`) (`KismetMathLibrary.MakeVector` (`self.SpeedH`)) false false)
            (set `self.SpeedH` (`KismetMathLibrary.Lerp` (`self.SpeedH`) 0.0 0.2))
            (`self.TeleportRows`)
            (else
              (`self.SnapToPosition`)))
          (if (>= (`KismetMathLibrary.Abs` (`self.SpeedV`)) 0.5)
            (`|ExecutionSequence`
              (:`then_0`
                (bind _newparam_2 (`self.TestLevelRowHeight`))
                (if _newparam_2
                  (`/Engine/EditorBlueprintResources/StandardMacros.IsValid` (`self.SelectedRowLevels`)
                    (:`Is Valid`
                      (`SceneComponent.K2_AddRelativeLocation` (`self.SelectedRowLevels`) (`KismetMathLibrary.MakeVector` 0.0 0.0 (`self.SpeedV`)) false false)
                      (set `self.SpeedV` (`KismetMathLibrary.Lerp` (`self.SpeedV`) 0.0 0.2)))
                    (:`Is Not Valid`
                      (set `self.SpeedV` 0.0 :!label _label)))
                  (else
                    (goto _label)))))
            (else
              (`self.LevelSnapToPosition`))))))
    (:`then_1`
      ;[1 1 1] Sets selected row based on distance - also sets visibility
      (for _array_element (`self.rows`)
        (bind _returnvalue (`SceneComponent.GetChildComponent` _array_element 0))
        (bind _returnvalue_2 (< (`KismetMathLibrary.Vector_Distance` (`SceneComponent.RelativeLocation` _array_element)) 70.0))
        (`SceneComponent.SetVisibility` _returnvalue _returnvalue_2 true)
        (if (and _returnvalue_2 (!= _array_element (`self.SelectedRoww`)))
          (set `self.SelectedRoww` _array_element)
          (set `self.SelectedRowLevels` _returnvalue)
          (if (== (`self.SelectedRoww`) (`self.Housing Selected`))
            (set `self.CurrentBuildingType` "NewEnumerator0")
            (elif (== (`self.SelectedRoww`) (`self.Storage Selected`))
              (set `self.CurrentBuildingType` "NewEnumerator1")
              (elif (== (`self.SelectedRoww`) (`self.Shops Selected`))
                (set `self.CurrentBuildingType` "NewEnumerator2")
                (elif (== (`self.SelectedRoww`) (`self.Clinic Selected`))
                  (set `self.CurrentBuildingType` "NewEnumerator3")
                  (elif (== (`self.SelectedRoww`) (`self.Research Selected`))
                    (set `self.CurrentBuildingType` "NewEnumerator4"))))))))
      (for (_array_element_2 _array_index) (`self.LevelSnapPoints`)
        (if (and (< (`KismetMathLibrary.Vector_Distance` (`SceneComponent.RelativeLocation` _array_element_2) (`SceneComponent.RelativeLocation` (`self.SelectedRowLevels`))) 70.0) (!= _array_element_2 (`self.SelectedRoww`)))
          (set `self.Level` _array_index))))))

(fn `LevelSnapToPosition`
  (locals (LerpPos :type "Float (double-precision)") (Distance :type "Float (double-precision)"))
  (bind (_relativelocation_x _relativelocation_y _relativelocation_z) (`KismetMathLibrary.BreakVector` (`SceneComponent.RelativeLocation` (`self.SelectedRowLevels`))))
  (`/Engine/EditorBlueprintResources/StandardMacros.IsValid` (`self.SelectedRowLevels`)
    (:`Is Valid`
      (set `local.LerpPos` 9999.0)
      (set `local.Distance` 9999.0)
      (for _array_element (`self.LevelSnapPoints`)
        (bind _relativelocation (`SceneComponent.RelativeLocation` _array_element))
        (bind _returnvalue (`KismetMathLibrary.Vector_Distance` _relativelocation (`KismetMathLibrary.MakeVector` _relativelocation_x _relativelocation_y _relativelocation_z)))
        (if (< _returnvalue (`local.Distance`))
          (set `local.Distance` _returnvalue)
          (set `local.LerpPos` (.z _relativelocation))))
      (`SceneComponent.K2_SetRelativeLocation` (`self.SelectedRowLevels`) (`KismetMathLibrary.MakeVector` _relativelocation_x _relativelocation_y (`KismetMathLibrary.Lerp` _relativelocation_z (`local.LerpPos`) 0.1)) false false))))

(fn `SnapToPosition`
  (locals (LerpPos :type "Float (double-precision)") (Distance :type "Float (double-precision)"))
  (for _array_element (`self.rows`)
    (set `local.LerpPos` 9999.0)
    (set `local.Distance` 9999.0)
    (for _array_element_2 (`self.BuildingSnapPoints`)
      (bind _relativelocation (`SceneComponent.RelativeLocation` _array_element_2))
      (bind (_relativelocation_x _relativelocation_y _relativelocation_z) (`KismetMathLibrary.BreakVector` (`SceneComponent.RelativeLocation` _array_element)))
      (bind _returnvalue (`KismetMathLibrary.Vector_Distance` _relativelocation (`KismetMathLibrary.MakeVector` _relativelocation_x _relativelocation_y _relativelocation_z)))
      (if (< _returnvalue (`local.Distance`))
        (set `local.Distance` _returnvalue)
        (set `local.LerpPos` (.x _relativelocation))))
    (`SceneComponent.K2_SetRelativeLocation` _array_element (`KismetMathLibrary.MakeVector` (`KismetMathLibrary.Lerp` _relativelocation_x (`local.LerpPos`) 0.1) _relativelocation_y _relativelocation_z) false false)))

(fn `TeleportRows`
  (locals (LeftPos :type Integer) (RightPos :type Integer))
  ;[1 1 1] Teleports Row if it moves out of bounds
  (for _array_element (`self.rows`)
    (bind _relativelocation_x (`KismetMathLibrary.BreakVector` (`SceneComponent.RelativeLocation` _array_element)))
    (if (> _relativelocation_x 375.0)
      (bind (_relativelocation_x_2 _relativelocation_y _relativelocation_z) (`KismetMathLibrary.BreakVector` (`SceneComponent.RelativeLocation` _array_element)))
      (`SceneComponent.K2_SetRelativeLocation` _array_element (`KismetMathLibrary.MakeVector` (- _relativelocation_x 750.0) _relativelocation_y _relativelocation_z) false false)
      (`KismetSystemLibrary.PrintString` "Hello")
      (elif (< _relativelocation_x -375.0)
        (`SceneComponent.K2_SetRelativeLocation` _array_element (`KismetMathLibrary.MakeVector` (+ _relativelocation_x 750.0) _relativelocation_y _relativelocation_z) false false)))))

(fn `TestLevelRowHeight`
  (returns (NewParam :type Boolean))
  (locals (TopPos :type "Float (double-precision)") (BottomPos :type "Float (double-precision)"))
  (bind _selectedrowlevels (`self.SelectedRowLevels`))
  (bind (_relativelocation_x _relativelocation_y _relativelocation_z) (`KismetMathLibrary.BreakVector` (`SceneComponent.RelativeLocation` (`self.PosLevel4`))))
  (bind (_relativelocation_x_2 _relativelocation_y_2 _relativelocation_z_2) (`KismetMathLibrary.BreakVector` (`SceneComponent.RelativeLocation` _selectedrowlevels)))
  (bind (_relativelocation_x_3 _relativelocation_y_3 _relativelocation_z_3) (`KismetMathLibrary.BreakVector` (`SceneComponent.RelativeLocation` (`self.PosLevel1`))))
  (set `local.TopPos` _relativelocation_z_3)
  (set `local.BottomPos` _relativelocation_z)
  (`/Engine/EditorBlueprintResources/StandardMacros.IsValid` _selectedrowlevels
    (:`Is Valid`
      (if (`KismetMathLibrary.BooleanNOR` (> _relativelocation_z_2 (`local.TopPos`)) (< _relativelocation_z_2 (`local.BottomPos`)))
        (return true)
        (else
          (`SceneComponent.K2_SetRelativeLocation` _selectedrowlevels (`KismetMathLibrary.MakeVector` _relativelocation_x_2 _relativelocation_y_2 (`KismetMathLibrary.FClamp` _relativelocation_z_2 (`local.BottomPos`) (`local.TopPos`))) false false))))
    (:`Is Not Valid`
      _))
  (return false))

(fn `UserConstructionScript`)